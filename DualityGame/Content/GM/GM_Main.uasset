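; GM_Main, by its name the game mode, bootstraps the player controller and character at BeginPlay.
; It removes the initial player without destroying its pawn, creates a new local player and stores its controller as PC_Main.
; It then spawns a C_PlayerChar with collision handling set to always spawn.
; An explicit init chain passes itself and the character to the controller, then itself to the character.
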(event EventBeginPlay
  (CallFunction|CreateController)
  (CallFunction|CreatePlayer)
  (CallFunction|InitChain))

(fn ConstructionScript)

(fn CreateController
  (Class|GameplayStatics|RemovePlayer (Game|GetPlayerController 0) false)
  (bind _returnvalue (Class|GameplayStatics|CreatePlayer -1))
  (Variables|Default|SetController (.AsPC%20Main (Utilities|Casting|CastToPC_Main _returnvalue))))

(fn CreatePlayer
  (bind _returnvalue (Game|SpawnActorfromClass "/Game/C_PlayerChar.C_PlayerChar_C" (Math|Transform|MakeTransform "0, 0, 0" "0, 0, 0" "1,1,1") "AlwaysSpawn" 0 0))
  (Variables|Default|SetCharacter _returnvalue))

(fn InitChain
  (Default|InitController (Variables|Default|GetController) self (Variables|Default|GetCharacter))
  (Default|InitCharacter (Variables|Default|GetCharacter) self))