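; PC_Main is the main player controller, driving a character along a single movement axis under a separately supplied camera.
; InitController stores the game mode, character and camera references, then possesses the character and makes the camera the view target.
; Input events forward move, jump start/stop and action to the character.
; Each Swap release uses a FlipFlop to alternate the character between two enum states.
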(event Custom|InitController
  (params (GMref :type GM%20Main%20Object%20Reference) (CharRef :type C%20Player%20Char%20Object%20Reference) (Camera :type BP%20Camera%20Actor%20Object%20Reference))
  (Variables|Default|SetGMref GMref)
  (Variables|Default|SetCameraRef Camera)
  (bind _output_get (Variables|Default|SetChar%20Ref CharRef))
  (Pawn|Possess _output_get)
  (Game|Player|SetViewTargetwithBlend (Variables|Default|GetCameraRef) 0.0 "VTBlend_Linear" 0.0 false))

(event Input|ActionEvents|InputActionSwap
  (params (Key :type Key%20Structure :default "None"))
  (bind _char_ref (Variables|Default|GetChar%20Ref))
  (:Released
    (Utilities|FlowControl|FlipFlop
      (:A
        (Default|Swap _char_ref "NewEnumerator1"))
      (:B
        (Default|Swap _char_ref "NewEnumerator0")))))

(event Input|ActionEvents|InputActionJump
  (params (Key :type Key%20Structure :default "None"))
  (bind _char_ref (Variables|Default|GetChar%20Ref))
  ;[0.03649 1 0] Inputs
  (:Pressed
    (Default|StartJump _char_ref))
  (:Released
    (Default|StopJump _char_ref)))

(event Input|ActionEvents|InputActionAction
  (params (Key :type Key%20Structure :default "None"))
  ;[0.03649 1 0] Inputs
  (:Released
    (Default|Action (Variables|Default|GetChar%20Ref))))

(event Input|AxisEvents|InputAxisMoveRight
  (params (AxisValue :type Float%20%28single-precision%29))
  (Default|Move (Variables|Default|GetChar%20Ref) AxisValue))

(fn ConstructionScript)