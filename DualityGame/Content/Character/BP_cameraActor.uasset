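; Camera actor that auto-scrolls endlessly along +X, carrying a boundary of death zones and a cloud spawner.
; InitCamera spawns and attaches death zones below, left, right and above, then starts movement and attaches an initialized BP_CloudSpawner.
; A looping timer lerps the location in fixed 500-unit segments, restarting from each endpoint.
; The upper zone overwrites the DeathZoneRight reference.
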(event Custom|StartCameraMovement
  (Transformation|SetActorLocation (Math|Vector|Lerp(Vector) (Variables|Default|GetActorLocation) (+ (Variables|Default|GetActorLocation) "500.000000,0.000000, 0") (Variables|Default|GetCameraAlpha)) true false)
  (bind _output_get (Variables|Default|SetCameraAlpha (+ (Variables|Default|GetCameraAlpha) 0.001)))
  (if (>= _output_get 1.0)
    (Utilities|Time|ClearandInvalidateTimerbyHandle (Variables|Default|GetCameraTimer))
    (Variables|Default|SetCameraAlpha 0.0)
    (CallFunction|StartCamera)))

(event Custom|StartCamera
  (bind _returnvalue (Utilities|Time|SetTimerbyEvent (delegate Custom|StartCameraMovement) 0.001 true))
  (Variables|Default|SetCameraTimer _returnvalue)
  (Variables|Default|SetActorLocation (Transformation|GetActorLocation)))

(event Custom|InitCamera
  (CallFunction|AddDeathZones)
  (CallFunction|StartCamera)
  (bind _returnvalue (Game|SpawnActorfromClass "/Game/Blueprint/BP_CloudSpawner.BP_CloudSpawner_C" (Math|Transform|MakeTransform (+ (Transformation|GetActorLocation) "7000.000000,-10300.000000,1000.000000") "0, 0, 0" "1,1,1") "Undefined" 0 0))
  (bind _output_get (Variables|Default|SetCloudSpawner _returnvalue))
  (Transformation|AttachActorToActor _output_get self "None" "KeepWorld" "KeepRelative" "KeepRelative" true)
  (Default|InitcloudSpawner _output_get))

(fn ConstructionScript)

(fn AddDeathZones
  (Utilities|FlowControl|Sequence
    (:then_0
      ;[1 1 1] Lower
      (bind _returnvalue (Game|SpawnActorfromClass "/Game/Blueprint/BP_DeathZone.BP_DeathZone_C" (Math|Transform|MakeTransform (- (Transformation|GetActorLocation) "0, 0,1000.000000") "0, 0, 0" "1,1,1") "Undefined" 0 0))
      (bind _output_get (Variables|Default|SetDeathZoneLower _returnvalue))
      (Transformation|AttachActorToActor _output_get self "None" "KeepWorld" "KeepWorld" "KeepRelative" true))
    (:then_1
      ;[1 1 1] Left
      (bind _returnvalue_2 (Game|SpawnActorfromClass "/Game/Blueprint/BP_DeathZone.BP_DeathZone_C" (Math|Transform|MakeTransform (- (Transformation|GetActorLocation) "1500.000000, 0,0.000000") "90.000000,0.000000, 0" "1,1,1") "Undefined" 0 0))
      (bind _output_get_2 (Variables|Default|SetDeathZoneLeft _returnvalue_2))
      (Transformation|AttachActorToActor _output_get_2 self "None" "KeepWorld" "KeepWorld" "KeepRelative" true))
    (:then_2
      ;[1 1 1] Right
      (bind _returnvalue_3 (Game|SpawnActorfromClass "/Game/Blueprint/BP_DeathZone.BP_DeathZone_C" (Math|Transform|MakeTransform (- (Transformation|GetActorLocation) "-1600.000000, 0,0.000000") "90.000000,0.000000, 0" "1,1,1") "Undefined" 0 0))
      (bind _output_get_3 (Variables|Default|SetDeathZoneRight _returnvalue_3))
      (Transformation|AttachActorToActor _output_get_3 self "None" "KeepWorld" "KeepWorld" "KeepRelative" true))
    (:then_3
      ;[1 1 1] Upper
      (bind _returnvalue_4 (Game|SpawnActorfromClass "/Game/Blueprint/BP_DeathZone.BP_DeathZone_C" (Math|Transform|MakeTransform (- (Transformation|GetActorLocation) "0.000000, 0,-900.000000") "0, 0, 0" "1,1,1") "Undefined" 0 0))
      (bind _output_get_4 (Variables|Default|SetDeathZoneRight _returnvalue_4))
      (Transformation|AttachActorToActor _output_get_4 self "None" "KeepWorld" "KeepWorld" "KeepRelative" true))))