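; Collectable goo orb that awards score only to a player whose size matches its own.
; On BeginPlay it randomly becomes Small or Large with even odds, setting the sphere's material and scale to match.
; On sphere overlap it fetches the player through GetPlayerMessage and compares sizes.
; A match adds points, plays a pickup sound and destroys the orb.
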(event OnComponentBeginOverlap(Sphere)
  (params (OverlappedComponent :type Primitive%20Component%20Object%20Reference) (OtherActor :type Actor%20Object%20Reference) (OtherComp :type Primitive%20Component%20Object%20Reference) (OtherBodyIndex :type Integer) (bFromSweep :type Boolean) (SweepResult :type Hit%20Result%20Structure%20%28by%20ref%29))
  (bind _playerref (Class|BPIObstacle|GetPlayer(Message) OtherActor))
  (Utilities|IsValid _playerref
    (:Is%20Valid
      (if (== (Variables|/Game/Character/C_PlayerChar.C_PlayerChar_C|GetSize _playerref) (Variables|Default|GetSelection))
        (Default|AddtoScore _playerref 1000)
        (Audio|PlaySoundatLocation "/Game/SoundEffects/sfxOrbPickupsIfThePickupsAreNotCommon_Cue.sfxOrbPickupsIfThePickupsAreNotCommon_Cue" (Transformation|GetActorLocation) "0, 0, 0" 1.0 1.0 0.0 0 0 0)
        (Actor|DestroyActor)))))

(event EventBeginPlay
  (bind _sphere1 (Variables|Default|GetSphere1))
  (bind _output_get (Variables|Default|SetSelection (select (Math|Random|RandomBoolwithWeight 0.5) "NewEnumerator1" "NewEnumerator0")))
  (switch Utilities|FlowControl|Switch|SwitchonE_Size _output_get
    (:NewEnumerator0
      (Rendering|Material|SetMaterial _sphere1 0 "/Game/Art/Meshes/Props/Collectable/IN_Goo_1.IN_Goo_1")
      (Transformation|SetWorldScale3D _sphere1 "2.000000,2.000000,2.000000"))
    (:NewEnumerator1
      (Rendering|Material|SetMaterial _sphere1 0 "/Game/Art/Meshes/Props/Collectable/IN_Goo_2.IN_Goo_2")
      (Transformation|SetWorldScale3D _sphere1 "1.000000,1.000000,1.000000"))))

(fn ConstructionScript)