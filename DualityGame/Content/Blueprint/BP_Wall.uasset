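; BP_Wall is a spline-driven modular wall that builds itself in the Construction Script from stone-brick bridge meshes.
; It steps along the spline at a Spacing interval, adding a start piece first, an end piece at the last whole step and middle pieces between, all as mesh instances.
; Each instance takes its slope and bank from the spline with axes swapped, while yaw stays fixed, ignoring horizontal curves.
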(fn ConstructionScript
  (bind _startpiece (Variables|Default|GetStartPiece))
  (bind _endpiece (Variables|Default|GetEndPiece))
  (bind _spline (Variables|Default|GetSpline))
  (bind _middlepiece (Variables|Default|GetMiddlePiece))
  (Utilities|FlowControl|Sequence
    (:then_0
      (Rendering|Material|SetMaterial _middlepiece 0 "/Game/Materials/StoneBrick/M_StoneBrick.M_StoneBrick")
      (Components|StaticMesh|SetStaticMesh _middlepiece "/Game/Art/Meshes/BridgePieces/BridgeModular_BridgePiece_Short.BridgeModular_BridgePiece_Short"))
    (:then_1
      (Rendering|Material|SetMaterial _startpiece 0 "/Game/Materials/StoneBrick/M_StoneBrick.M_StoneBrick")
      (Components|StaticMesh|SetStaticMesh _startpiece "/Game/Art/Meshes/BridgePieces/BridgeModular_BridgePiece_Start.BridgeModular_BridgePiece_Start"))
    (:then_2
      (Rendering|Material|SetMaterial _endpiece 0 "/Game/Materials/StoneBrick/M_StoneBrick.M_StoneBrick")
      (Components|StaticMesh|SetStaticMesh _endpiece "/Game/Art/Meshes/BridgePieces/BridgeModular_BridgePiece_End.BridgeModular_BridgePiece_End"))
    (:then_3
      (bind _output_get (Variables|Default|SetNumberOfInstances (Math|Float|Floor (/ (Spline|GetSplineLength (Variables|Default|GetSpline)) (Variables|Default|GetSpacing)))))
      (for _index (range 0 _output_get)
        (if (== _index 0)
          (Components|InstancedStaticMesh|AddInstance (Variables|Default|GetStartPiece) (Math|Transform|MakeTransform (Spline|GetLocationatDistanceAlongSpline _spline (* _index (Variables|Default|GetSpacing)) "Local") (Math|Rotator|MakeRotator (* (.pitch (Spline|GetRotationatDistanceAlongSpline _spline (* _index (Variables|Default|GetSpacing)) "Local")) -1.0) (.roll (Spline|GetRotationatDistanceAlongSpline _spline (* _index (Variables|Default|GetSpacing)) "Local")) -9e+01)))
          (elif (== _index _output_get)
            (Components|InstancedStaticMesh|AddInstance (Variables|Default|GetEndPiece) (Math|Transform|MakeTransform (Spline|GetLocationatDistanceAlongSpline _spline (* _index (Variables|Default|GetSpacing)) "Local") (Math|Rotator|MakeRotator (* (.pitch (Spline|GetRotationatDistanceAlongSpline _spline (* _index (Variables|Default|GetSpacing)) "Local")) -1.0) (.roll (Spline|GetRotationatDistanceAlongSpline _spline (* _index (Variables|Default|GetSpacing)) "Local")) -9e+01)))
            (else
              (Components|InstancedStaticMesh|AddInstance (Variables|Default|GetMiddlePiece) (Math|Transform|MakeTransform (Spline|GetLocationatDistanceAlongSpline _spline (* _index (Variables|Default|GetSpacing)) "Local") (Math|Rotator|MakeRotator (* (.pitch (Spline|GetRotationatDistanceAlongSpline _spline (* _index (Variables|Default|GetSpacing)) "Local")) -1.0) (.roll (Spline|GetRotationatDistanceAlongSpline _spline (* _index (Variables|Default|GetSpacing)) "Local")) -9e+01))))))))))