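; BP_PathwayObstacle is a pathway obstacle that stuns the player on overlap.
; When something enters its Box, it fetches a player reference from the other actor through GetPlayerMessage, then stores it and calls Stunned if it is valid.
; The construction script sizes the Box and sets and offsets the static mesh from variables, so one Blueprint covers different obstacle shapes.
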(event OnComponentBeginOverlap(Box)
  (params (OverlappedComponent :type Primitive%20Component%20Object%20Reference) (OtherActor :type Actor%20Object%20Reference) (OtherComp :type Primitive%20Component%20Object%20Reference) (OtherBodyIndex :type Integer) (bFromSweep :type Boolean) (SweepResult :type Hit%20Result%20Structure%20%28by%20ref%29))
  ;[1 1 1] OnCollide
  (bind _playerref (Class|BPIObstacle|GetPlayer(Message) OtherActor))
  (if (Utilities|IsValid _playerref)
    (bind _output_get (Variables|Default|SetPlayer%20Ref _playerref))
    (Default|Stunned _output_get)))

(fn ConstructionScript
  (bind _staticmesh (Variables|Default|GetStaticMesh))
  (Components|Box|SetBoxExtent (Variables|Default|GetBox) (Variables|Default|GetIn%20Box%20Extent) true)
  (Components|StaticMesh|SetStaticMesh _staticmesh (Variables|Default|GetMeshToSet))
  (Transformation|AddLocalOffset _staticmesh (Variables|Default|GetMesh%20Offset) false false))

(fn GetPlayer)