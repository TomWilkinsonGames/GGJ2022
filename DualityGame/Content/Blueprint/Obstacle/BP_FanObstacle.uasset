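; BP_FanObstacle is a fan obstacle that pushes players inside its Box trigger along world +Y.
; On overlap begin, it resolves the player through GetPlayerMessage, launches immediately and starts a looping timer that repeats the check.
; Each check calls LaunchCharacter with a fixed velocity unless the player's Size equals the first enum value, so that size is unaffected.
; Ending the overlap clears the timer.
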(event OnComponentBeginOverlap(Box)
  (params (OverlappedComponent :type Primitive%20Component%20Object%20Reference) (OtherActor :type Actor%20Object%20Reference) (OtherComp :type Primitive%20Component%20Object%20Reference) (OtherBodyIndex :type Integer) (bFromSweep :type Boolean) (SweepResult :type Hit%20Result%20Structure%20%28by%20ref%29))
  (bind _playerref (Class|BPIObstacle|GetPlayer(Message) OtherActor))
  (if (Utilities|IsValid _playerref)
    (bind _returnvalue (Utilities|Time|SetTimerbyEvent (delegate Custom|CheckFanEvent) 0.1 true))
    (Variables|Default|SetCheckFan _returnvalue)
    (if (not (Utilities|Enum|Equal(Enum) (Variables|/Game/Character/C_PlayerChar.C_PlayerChar_C|GetSize _playerref) "NewEnumerator0"))
      (Character|LaunchCharacter _playerref "0,2000.000000, 0" false false))))

(event OnComponentEndOverlap(Box)
  (params (OverlappedComponent :type Primitive%20Component%20Object%20Reference) (OtherActor :type Actor%20Object%20Reference) (OtherComp :type Primitive%20Component%20Object%20Reference) (OtherBodyIndex :type Integer))
  (bind _playerref (Class|BPIObstacle|GetPlayer(Message) OtherActor))
  (if (Utilities|IsValid _playerref)
    (if (Utilities|Time|IsValidTimerHandle (Variables|Default|GetCheckFan))
      (Utilities|Time|ClearandInvalidateTimerbyHandle (Variables|Default|GetCheckFan)))))

(event Custom|CheckFanEvent
  (if (not (Utilities|Enum|Equal(Enum) (Variables|/Game/Character/C_PlayerChar.C_PlayerChar_C|GetSize (stale OnComponentBeginOverlap(Box) _playerref)) "NewEnumerator0"))
    (Character|LaunchCharacter (stale OnComponentBeginOverlap(Box) _playerref) "0,2000.000000, 0" false false)))

(fn ConstructionScript)