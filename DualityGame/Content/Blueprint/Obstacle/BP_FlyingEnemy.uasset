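; Flying enemy obstacle that, when Moves is enabled, travels vertically with a spinning fan and removes itself after a fixed lifetime.
; On BeginPlay, a timeline lerps the root from its start Z to MoveDistance as an absolute world height, rotating the fan each update.
; Timers replay the flying sound and later destroy the actor.
; A second timeline plays with no logic attached.
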(event Custom|Destroy
  (if (Utilities|IsValid self)
    (Actor|DestroyActor)))

(event Custom|StartSound
  (Audio|PlaySoundatLocation "/Game/SoundEffects/sfxFlyingEnemy_Cue.sfxFlyingEnemy_Cue" (Transformation|GetActorLocation) "0, 0, 0" 1.0 1.0 0.0 0 0 0))

(event EventBeginPlay
  (if (Variables|Default|GetMoves?)
    (Variables|Default|SetStartLocation (Transformation|GetWorldLocation (Variables|Default|GetDefaultSceneRoot)))
    (Utilities|FlowControl|Sequence
      (:then_0
        (bind _newtrack_0 (Timeline|Timeline_0 Play)
          (:Update
            (Transformation|SetWorldLocation (Variables|Default|GetDefaultSceneRoot) (Math|Vector|Lerp(Vector) (Variables|Default|GetStartLocation) (Math|Vector|MakeVector (.X (Math|Vector|BreakVector (Variables|Default|GetStartLocation))) (.Y (Math|Vector|BreakVector (Variables|Default|GetStartLocation))) (Variables|Default|GetMoveDistance)) _newtrack_0) false false)
            (Transformation|AddLocalRotation (Variables|Default|GetBP_FlyingEnemyFan) "0.000000,5.000000,0.000000" false false))))
      (:then_1
        (Timeline|Timeline_1 Play))
      (:then_2
        (Utilities|Time|SetTimerbyEvent (delegate Custom|StartSound) 1.5 true))
      (:then_3
        (Utilities|Time|SetTimerbyEvent (delegate Custom|Destroy) 2e+01)))))

(fn ConstructionScript
  (|CallParentFunction))