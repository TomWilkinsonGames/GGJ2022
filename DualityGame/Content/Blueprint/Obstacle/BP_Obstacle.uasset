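; BP_Obstacle is an obstacle that kills the player on contact unless they are in the movement state it requires.
; Its construction script applies a configurable mesh, and a box overlap gets the player through a GetPlayerMessage call on the overlapping actor.
; A switch on RequiredPlayerState lets matching Slide or Smash players pass with debug text, while Run obstacles always trigger PlayerDeathEvent.
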(event OnComponentBeginOverlap(Box)
  (params (OverlappedComponent :type Primitive%20Component%20Object%20Reference) (OtherActor :type Actor%20Object%20Reference) (OtherComp :type Primitive%20Component%20Object%20Reference) (OtherBodyIndex :type Integer) (bFromSweep :type Boolean) (SweepResult :type Hit%20Result%20Structure%20%28by%20ref%29))
  ;[1 1 1] OnCollide
  (bind _playerref (Class|BPIObstacle|GetPlayer(Message) OtherActor))
  (if (Utilities|IsValid _playerref)
    (Variables|Default|SetPlayer%20Ref _playerref)
    (switch Utilities|FlowControl|Switch|SwitchonE_PlayerState (Variables|Default|GetRequiredPlayerState)
      (:NewEnumerator0
        (if (Utilities|Enum|Equal(Enum) (Variables|/Game/Character/C_PlayerChar.C_PlayerChar_C|GetPlayerStates (Variables|Default|GetPlayer%20Ref)) "NewEnumerator0")
          (Development|PrintString "YOU SLIDE UNDER THAT NICE!" true true "(R=0.000000,G=1.000000,B=0.000000,A=1.000000)")
          (else
            (Default|PlayerDeathEvent (Variables|Default|GetPlayer%20Ref)))))
      (:NewEnumerator1
        (if (Utilities|Enum|Equal(Enum) (Variables|/Game/Character/C_PlayerChar.C_PlayerChar_C|GetPlayerStates (Variables|Default|GetPlayer%20Ref)) "NewEnumerator1")
          (Development|PrintString "YOU SMASHED THROUGH THAT NICE!" true true "(R=0.000000,G=1.000000,B=0.000000,A=1.000000)")
          (else
            (Default|PlayerDeathEvent (Variables|Default|GetPlayer%20Ref))
            (Development|PrintString "UH OH YOU DIDNT SMASH" true true "(R=0.000000,G=1.000000,B=0.000000,A=1.000000)"))))
      (:NewEnumerator2
        (Default|PlayerDeathEvent (Variables|Default|GetPlayer%20Ref))))))

(fn ConstructionScript
  (Components|StaticMesh|SetStaticMesh (Variables|Default|GetStaticMesh) (Variables|Default|GetMeshToSet)))

(fn GetPlayer)