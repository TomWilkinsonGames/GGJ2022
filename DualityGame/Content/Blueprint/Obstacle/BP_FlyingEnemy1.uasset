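; BP_FlyingEnemy1 is a flying enemy obstacle that, when Moves is set, travels along world X, plays an electric sound and expires.
; On BeginPlay a timeline lerps the root from its start location to MoveDistance, used as an absolute X coordinate rather than an offset.
; A second timeline plays with nothing wired to it.
; The sound plays immediately and repeats on a looping timer, while another timer destroys the actor after 20 seconds.
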(event Custom|Destroy
  (if (Utilities|IsValid self)
    (Actor|DestroyActor)))

(event Custom|StartSound
  (Audio|PlaySoundatLocation "/Game/SoundEffects/sfxElectricEnemy_Cue.sfxElectricEnemy_Cue" (Transformation|GetActorLocation) "0, 0, 0" 1.0 1.0 0.0 0 0 0))

(event EventBeginPlay
  (if (Variables|Default|GetMoves?)
    (Variables|Default|SetStartLocation (Transformation|GetWorldLocation (Variables|Default|GetDefaultSceneRoot)))
    (Utilities|FlowControl|Sequence
      (:then_0
        (bind _newtrack_0 (Timeline|Timeline_0 Play)
          (:Update
            (Transformation|SetWorldLocation (Variables|Default|GetDefaultSceneRoot) (Math|Vector|Lerp(Vector) (Variables|Default|GetStartLocation) (Math|Vector|MakeVector (Variables|Default|GetMoveDistance) (.Y (Math|Vector|BreakVector (Variables|Default|GetStartLocation))) (.Z (Math|Vector|BreakVector (Variables|Default|GetStartLocation)))) _newtrack_0) false false))))
      (:then_1
        (Timeline|Timeline_1 Play))
      (:then_2
        (Utilities|Time|SetTimerbyEvent (delegate Custom|StartSound) 5.0 true)
        (Audio|PlaySoundatLocation "/Game/SoundEffects/sfxElectricEnemy_Cue.sfxElectricEnemy_Cue" (Transformation|GetActorLocation) "0, 0, 0" 1.0 1.0 0.0 0 0 0))
      (:then_3
        (Utilities|Time|SetTimerbyEvent (delegate Custom|Destroy) 2e+01)))))

(fn ConstructionScript
  (|CallParentFunction))