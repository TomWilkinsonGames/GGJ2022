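; BP_GlassFloor is an obstacle floor that breaks under the player unless their Size matches one specific enum state.
; Entering the Box trigger checks Size at once and starts a looping timer that rechecks it, catching size changes while on the glass.
; Leaving the trigger clears the timer.
; Breaking simply hides the Glass component and disables its collision, with no restore logic.
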(event OnComponentBeginOverlap(Box)
  (params (OverlappedComponent :type Primitive%20Component%20Object%20Reference) (OtherActor :type Actor%20Object%20Reference) (OtherComp :type Primitive%20Component%20Object%20Reference) (OtherBodyIndex :type Integer) (bFromSweep :type Boolean) (SweepResult :type Hit%20Result%20Structure%20%28by%20ref%29))
  (bind _playerref (Class|BPIObstacle|GetPlayer(Message) OtherActor))
  (Variables|Default|SetPlayer%20Ref _playerref)
  (if (Utilities|IsValid (Variables|Default|GetPlayer%20Ref))
    (bind _returnvalue (Utilities|Time|SetTimerbyEvent (delegate Custom|CheckFloorEvent) 0.1 true))
    (Variables|Default|SetCheckFloor _returnvalue)
    (if (not (Utilities|Enum|Equal(Enum) (Variables|/Game/Character/C_PlayerChar.C_PlayerChar_C|GetSize (Variables|Default|GetPlayer%20Ref)) "NewEnumerator1"))
      (CallFunction|Break))))

(event OnComponentEndOverlap(Box)
  (params (OverlappedComponent :type Primitive%20Component%20Object%20Reference) (OtherActor :type Actor%20Object%20Reference) (OtherComp :type Primitive%20Component%20Object%20Reference) (OtherBodyIndex :type Integer))
  (bind _playerref (Class|BPIObstacle|GetPlayer(Message) OtherActor))
  (if (Utilities|IsValid _playerref)
    (Utilities|Time|ClearandInvalidateTimerbyHandle (Variables|Default|GetCheckFloor))))

(event Custom|Break
  (Development|SetHiddeninGame (Variables|Default|GetGlass) true false)
  (Collision|SetCollisionEnabled (Variables|Default|GetGlass) "NoCollision"))

(event Custom|CheckFloorEvent
  (bind _playerref (Class|BPIObstacle|GetPlayer(Message) (Game|GetPlayerCharacter 0)))
  (Variables|Default|SetPlayer%20Ref _playerref)
  (if (not (Utilities|Enum|Equal(Enum) (Variables|/Game/Character/C_PlayerChar.C_PlayerChar_C|GetSize (Variables|Default|GetPlayer%20Ref)) "NewEnumerator1"))
    (CallFunction|Break)))

(fn ConstructionScript)