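; A wooden obstacle that a large player smashes apart and that stuns a small player on contact.
; Box overlap gets the other actor's player via GetPlayerMessage and branches on its Size.
; A bash plays a wood-smash sound and swaps the intact Sign for hidden pre-fractured wall pieces, enabling their collision and gravity.
; A timer destroys the actor shortly afterwards.
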(event OnComponentBeginOverlap(Box)
  (params (OverlappedComponent :type Primitive%20Component%20Object%20Reference) (OtherActor :type Actor%20Object%20Reference) (OtherComp :type Primitive%20Component%20Object%20Reference) (OtherBodyIndex :type Integer) (bFromSweep :type Boolean) (SweepResult :type Hit%20Result%20Structure%20%28by%20ref%29))
  (bind _playerref (Class|BPIObstacle|GetPlayer(Message) OtherActor))
  (Utilities|IsValid _playerref
    (:Is%20Valid
      (switch Utilities|FlowControl|Switch|SwitchonE_Size (Variables|/Game/Character/C_PlayerChar.C_PlayerChar_C|GetSize _playerref)
        (:NewEnumerator0
          (CallFunction|BASH))
        (:NewEnumerator1
          (Default|Stunned _playerref))))))

(event Custom|BASH
  (bind _sign (Variables|Default|GetSign))
  (Audio|PlaySoundatLocation "/Game/SoundEffects/sfxWoodSmash_Cue.sfxWoodSmash_Cue" (Transformation|GetActorLocation) "0, 0, 0" 1.0 1.0 0.0 0 0 0)
  (Development|SetHiddeninGame _sign true false)
  (Collision|SetCollisionEnabled _sign "NoCollision")
  (for _array_element (Utilities|Array|MakeArray (Variables|Default|GetWooden_Wall_Planks2) (Variables|Default|GetWooden_Wall_Object004) (Variables|Default|GetWooden_Wall_Octogon) (Variables|Default|GetWooden_Wall_P) (Variables|Default|GetWooden_Wall_Planks) (Variables|Default|GetWooden_Wall_Planks1) (Variables|Default|GetWooden_Wall_Planks12) (Variables|Default|GetWooden_Wall_Planks13) (Variables|Default|GetWooden_Wall_Planks14) (Variables|Default|GetWooden_Wall_Planks15) (Variables|Default|GetWooden_Wall_Planks16) (Variables|Default|GetWooden_Wall_O) (Variables|Default|GetWooden_Wall_Planks3) (Variables|Default|GetWooden_Wall_Planks4) (Variables|Default|GetWooden_Wall_Planks5) (Variables|Default|GetWooden_Wall_Planks6) (Variables|Default|GetWooden_Wall_Planks7) (Variables|Default|GetWooden_Wall_Planks8) (Variables|Default|GetWooden_Wall_S) (Variables|Default|GetWooden_Wall_Struts) (Variables|Default|GetWooden_Wall_Struts10) (Variables|Default|GetWooden_Wall_Struts11) (Variables|Default|GetWooden_Wall_Struts9))
    (Collision|SetCollisionEnabled _array_element "QueryAndPhysics")
    (Physics|SetEnableGravity _array_element true)
    (Development|SetHiddeninGame _array_element false false))
  (Utilities|Time|SetTimerbyEvent (delegate Custom|Delete) 15.0))

(event Custom|Delete
  (Actor|DestroyActor))

(fn ConstructionScript)