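; Modular bridge Blueprint that lays start, middle and end pieces along a spline in the construction script, with no runtime logic.
; It divides spline length by Spacing, then adds instances to three instanced mesh components, with the first and last indices getting the end caps.
; Each piece takes its local location and remapped pitch and roll from the spline, while yaw stays fixed, so pieces do not turn with horizontal bends.
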(event EventBeginPlay)

(event Collision|EventActorBeginOverlap
  (params (OtherActor :type Actor%20Object%20Reference)))

(event EventTick
  (params (DeltaSeconds :type Float%20%28single-precision%29)))

(fn ConstructionScript
  (bind _spline (Variables|Default|GetSpline))
  (Utilities|FlowControl|Sequence
    (:then_0
      (Components|StaticMesh|SetStaticMesh (Variables|Default|GetMiddlePiece) "/Game/Art/Meshes/BridgePieces/BridgeModular_BridgePiece_Short.BridgeModular_BridgePiece_Short"))
    (:then_1
      (Components|StaticMesh|SetStaticMesh (Variables|Default|GetStartPiece) "/Game/Art/Meshes/BridgePieces/BridgeModular_BridgePiece_Start.BridgeModular_BridgePiece_Start"))
    (:then_2
      (Components|StaticMesh|SetStaticMesh (Variables|Default|GetEndPiece) "/Game/Art/Meshes/BridgePieces/BridgeModular_BridgePiece_End.BridgeModular_BridgePiece_End"))
    (:then_3
      (bind _output_get (Variables|Default|SetNumberOfInstances (Math|Float|Floor (/ (Spline|GetSplineLength (Variables|Default|GetSpline)) (Variables|Default|GetSpacing)))))
      (for _index (range 0 _output_get)
        (if (== _index 0)
          (Components|InstancedStaticMesh|AddInstance (Variables|Default|GetStartPiece) (Math|Transform|MakeTransform (Spline|GetLocationatDistanceAlongSpline _spline (* _index (Variables|Default|GetSpacing)) "Local") (Math|Rotator|MakeRotator (* (.pitch (Spline|GetRotationatDistanceAlongSpline _spline (* _index (Variables|Default|GetSpacing)) "Local")) -1.0) (.roll (Spline|GetRotationatDistanceAlongSpline _spline (* _index (Variables|Default|GetSpacing)) "Local")) -9e+01)))
          (elif (== _index _output_get)
            (Components|InstancedStaticMesh|AddInstance (Variables|Default|GetEndPiece) (Math|Transform|MakeTransform (Spline|GetLocationatDistanceAlongSpline _spline (* _index (Variables|Default|GetSpacing)) "Local") (Math|Rotator|MakeRotator (* (.pitch (Spline|GetRotationatDistanceAlongSpline _spline (* _index (Variables|Default|GetSpacing)) "Local")) -1.0) (.roll (Spline|GetRotationatDistanceAlongSpline _spline (* _index (Variables|Default|GetSpacing)) "Local")) -9e+01)))
            (else
              (Components|InstancedStaticMesh|AddInstance (Variables|Default|GetMiddlePiece) (Math|Transform|MakeTransform (Spline|GetLocationatDistanceAlongSpline _spline (* _index (Variables|Default|GetSpacing)) "Local") (Math|Rotator|MakeRotator (* (.pitch (Spline|GetRotationatDistanceAlongSpline _spline (* _index (Variables|Default|GetSpacing)) "Local")) -1.0) (.roll (Spline|GetRotationatDistanceAlongSpline _spline (* _index (Variables|Default|GetSpacing)) "Local")) -9e+01))))))))))