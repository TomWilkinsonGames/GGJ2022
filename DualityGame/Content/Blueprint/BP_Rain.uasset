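; BP_Rain is a weather actor that spawns recurring lightning emitters while IsRain is set.
; Tick relies on latent Delays to pace strikes, waiting a random few seconds, spawning a vertically stretched P_Lightning at world origin, then destroying it after another delay.
; The construction script sizes a Box from Extent, but spawning ignores it.
; Unconnected nodes hold an unused choice between lightning, fireflies and dandelion effects.
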(event EventTick
  (params (DeltaSeconds :type Float%20%28single-precision%29))
  (if (Variables|Default|GetIsRain)
    (Utilities|FlowControl|Delay (Math|Random|RandomFloatinRange 3.0 6.0))
    (bind _returnvalue (Effects|SpawnEmitteratLocation "/Game/ImporredAssets/AssetsWeWant/P_Lightning.P_Lightning" "0.000000, 0, 0" "0.000000, 0, 0" "0.250000,0.250000,5.000000"))
    (Utilities|FlowControl|Delay 6.0)
    (Utilities|IsValid _returnvalue
      (:Is%20Valid
        (Components|DestroyComponent _returnvalue)))))

(fn ConstructionScript
  (Components|Box|SetBoxExtent (Variables|Default|GetBox) (Variables|Default|GetExtent) true))