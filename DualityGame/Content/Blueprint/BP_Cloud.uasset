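; BP_Cloud is a short-lived cloud actor that drifts along negative X.
; On BeginPlay it picks one of three meshes, randomizes its scale and starts movement.
; A fast looping timer, rather than Tick, lerps the location in swept steps, restarting each completed segment from the current position for continuous drift.
; A separate one-shot timer later clears the movement timer and destroys the actor.
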(event Custom|MoveCloud
  (bind _returnvalue (Transformation|GetActorLocation))
  (bind _cloudstartlocation (Variables|Default|GetCloudStartLocation))
  (Transformation|SetActorLocation (Math|Vector|MakeVector (Math|Float|Lerp _cloudstartlocation (+ _cloudstartlocation -5e+02) (Variables|Default|GetAlpha)) (.y _returnvalue) (.z _returnvalue)) true false)
  (bind _output_get (Variables|Default|SetAlpha (+ (Variables|Default|GetAlpha) 0.001)))
  (if (>= _output_get 1.0)
    (Variables|Default|SetAlpha 0.0)
    (Utilities|Time|ClearandInvalidateTimerbyHandle (Variables|Default|GetCloudMoveTimer))
    (CallFunction|StartCloudMovement)))

(event Custom|Kill
  (bind _cloudmovetimer (Variables|Default|GetCloudMoveTimer))
  (if (Utilities|Time|IsValidTimerHandle _cloudmovetimer)
    (Utilities|Time|ClearandInvalidateTimerbyHandle _cloudmovetimer)
    (Actor|DestroyActor)))

(event Custom|StartCloudMovement
  (Variables|Default|SetCloudStartLocation (.x (Transformation|GetActorLocation)))
  (bind _returnvalue (Utilities|Time|SetTimerbyEvent (delegate Custom|MoveCloud) 0.001 true))
  (Variables|Default|SetCloudMoveTimer _returnvalue))

(event EventBeginPlay
  (Components|StaticMesh|SetStaticMesh (Variables|Default|GetCloudMesh) (Utilities|Select :Index (Math|Random|RandomIntegerinRange 0 2) :Option%200 (Variables|Default|GetCloud1) :Option%201 (Variables|Default|GetCloud2) :Option%202 (Variables|Default|GetCloud3)))
  (Transformation|SetWorldScale3D (Variables|Default|GetCloudMesh) (* (Variables|Default|GetNew%20Scale) (Math|Random|RandomFloatinRange 0.2 0.8)))
  (CallFunction|StartCloudMovement)
  (Utilities|Time|SetTimerbyEvent (delegate Custom|Kill) 15.0))

(fn ConstructionScript)