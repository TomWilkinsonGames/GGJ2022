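; BP_WallThick is a spline-driven construction tool that builds a thick modular wall from wide wall-block meshes.
; Its construction script divides the spline length by Spacing and adds instances to StartPiece, MiddlePiece and EndPiece for the first, intermediate and last positions.
; All three components use the same mesh.
; Blocks follow spline positions with a fixed offset and yaw, ignoring spline rotation, so they do not turn along curves.
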(fn ConstructionScript
  (Utilities|FlowControl|Sequence
    (:then_0
      (Components|StaticMesh|SetStaticMesh (Variables|Default|GetMiddlePiece) "/Game/Art/Meshes/BridgePieces/BridgeModular_WallBlock_Wide.BridgeModular_WallBlock_Wide"))
    (:then_1
      (Components|StaticMesh|SetStaticMesh (Variables|Default|GetStartPiece) "/Game/Art/Meshes/BridgePieces/BridgeModular_WallBlock_Wide.BridgeModular_WallBlock_Wide"))
    (:then_2
      (Components|StaticMesh|SetStaticMesh (Variables|Default|GetEndPiece) "/Game/Art/Meshes/BridgePieces/BridgeModular_WallBlock_Wide.BridgeModular_WallBlock_Wide"))
    (:then_3
      (bind _output_get (Variables|Default|SetNumberOfInstances (Math|Float|Floor (/ (Spline|GetSplineLength (Variables|Default|GetSpline)) (Variables|Default|GetSpacing)))))
      (for _index (range 0 _output_get)
        (if (== _index 0)
          (Components|InstancedStaticMesh|AddInstance (Variables|Default|GetStartPiece) (Math|Transform|MakeTransform (Math|Vector|MakeVector (.x (Spline|GetLocationatDistanceAlongSpline (Variables|Default|GetSpline) (* _index (Variables|Default|GetSpacing)) "Local")) (+ (.y (Spline|GetLocationatDistanceAlongSpline (Variables|Default|GetSpline) (* _index (Variables|Default|GetSpacing)) "Local")) 1e+01) (+ (.z (Spline|GetLocationatDistanceAlongSpline (Variables|Default|GetSpline) (* _index (Variables|Default|GetSpacing)) "Local")) -25.0)) (Math|Rotator|MakeRotator 0.0 0.0 -9e+01)))
          (elif (== _index _output_get)
            (Components|InstancedStaticMesh|AddInstance (Variables|Default|GetEndPiece) (Math|Transform|MakeTransform (Math|Vector|MakeVector (.x (Spline|GetLocationatDistanceAlongSpline (Variables|Default|GetSpline) (* _index (Variables|Default|GetSpacing)) "Local")) (+ (.y (Spline|GetLocationatDistanceAlongSpline (Variables|Default|GetSpline) (* _index (Variables|Default|GetSpacing)) "Local")) 1e+01) (+ (.z (Spline|GetLocationatDistanceAlongSpline (Variables|Default|GetSpline) (* _index (Variables|Default|GetSpacing)) "Local")) -25.0)) (Math|Rotator|MakeRotator 0.0 0.0 -9e+01)))
            (else
              (Components|InstancedStaticMesh|AddInstance (Variables|Default|GetMiddlePiece) (Math|Transform|MakeTransform (Math|Vector|MakeVector (.x (Spline|GetLocationatDistanceAlongSpline (Variables|Default|GetSpline) (* _index (Variables|Default|GetSpacing)) "Local")) (+ (.y (Spline|GetLocationatDistanceAlongSpline (Variables|Default|GetSpline) (* _index (Variables|Default|GetSpacing)) "Local")) 1e+01) (+ (.z (Spline|GetLocationatDistanceAlongSpline (Variables|Default|GetSpline) (* _index (Variables|Default|GetSpacing)) "Local")) -25.0)) (Math|Rotator|MakeRotator 0.0 0.0 -9e+01))))))))))