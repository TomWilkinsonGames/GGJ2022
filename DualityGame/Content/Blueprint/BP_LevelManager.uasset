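; Level manager that builds an endless strip of randomly chosen level tiles along X.
; A looping timer picks from Section01Levels, recursively re-picking any tile found in a short history of recent picks.
; Each pick loads as a soft-referenced level instance one TileLength past the last.
; Once the loaded count exceeds TilesAtOneTime, the oldest instance is unloaded and removed.
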(event Custom|SpawnTile
  (bind _recenttiles (Variables|Default|GetRecentTiles))
  (bind _output (CallFunction|PickRandomLevel))
  (bind _sameasprevious (CallFunction|CheckLevel))
  (if (not _sameasprevious)
    (Utilities|Array|Add (Variables|Default|GetRecentTiles) _output)
    (CallFunction|SpawnLevel _output)
    (if (>= (Utilities|Array|Length _recenttiles) 3)
      (Utilities|Array|RemoveIndex _recenttiles))))

(event Custom|SpawnLevel
  (params (Level :type World%20Soft%20Object%20Reference))
  (bind _output_get (Variables|Default|SetTileLocation (+ (Variables|Default|GetTileLength) (Variables|Default|GetTileLocation))))
  (bind _returnvalue (Class|LevelStreamingDynamic|LoadLevelInstancebySoftObjectPtr Level (Math|Vector|MakeVector _output_get 0.0 0.0) "0, 0, 0"))
  (bind _returnvalue_2 (Utilities|Array|Add (Variables|Default|GetLevelTiles) _returnvalue))
  (Variables|Default|SetIteration (+ (Variables|Default|GetIteration) 1))
  (if (>= _returnvalue_2 (Variables|Default|GetTilesAtOneTime))
    (Class|LevelStreaming|SetIsRequestingUnloadandRemoval (Utilities|Array|Get(acopy) (Variables|Default|GetLevelTiles)) true)
    (Utilities|Array|RemoveIndex (Variables|Default|GetLevelTiles))))

(event Custom|PickLevelAgain
  (bind _recenttiles (Variables|Default|GetRecentTiles))
  (bind _output (CallFunction|PickRandomLevel))
  (bind _sameasprevious (CallFunction|CheckLevel))
  (if (not _sameasprevious)
    (Utilities|Array|Add (Variables|Default|GetRecentTiles) _output)
    (CallFunction|SpawnLevel _output)
    (if (>= (Utilities|Array|Length _recenttiles) 3)
      (Utilities|Array|RemoveIndex _recenttiles))))

(event EventBeginPlay
  (CallFunction|SpawnTile)
  (Utilities|Time|SetTimerbyEvent (delegate Custom|SpawnTile) (Variables|Default|GetSpawnDelay) true))

(fn ConstructionScript)

(fn CheckLevel
  (if (Utilities|Array|ContainsItem (Variables|Default|GetRecentTiles) (Variables|Default|GetRandomLevel))
    (CallFunction|PickLevelAgain)
    (return true)
    (else
      (return false))))

(fn PickRandomLevel
  (bind _section01levels (Variables|Default|GetSection01Levels))
  (bind _output_get (Variables|Default|SetRandomLevel (Utilities|Array|Get(acopy) _section01levels (Math|Random|RandomIntegerinRange 0 (Utilities|Array|LastIndex _section01levels)))))
  (return _output_get))