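; BP_CloudSpawner spawns BP_Cloud actors at random points inside a box zone around its location.
; InitcloudSpawner starts a looping timer whose short interval is randomized once, when the timer is set.
; Each tick of that timer spawns a cloud within InBoxExtent and passes LevelBase as its Mesh.
; The construction script sizes the CloudSpawnZone box from the same extent.
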(event Custom|SpawnCloud
  (Game|SpawnActorfromClass "/Game/Blueprint/BP_Cloud.BP_Cloud_C" (Math|Transform|MakeTransform (+ (Transformation|GetActorLocation self) (Math|Random|RandomPointinBoundingBox "0, 0, 0" (Variables|Default|GetIn%20Box%20Extent))) "0, 0, 0" "1,1,1") "Undefined" 0 "/Game/Art/Meshes/LevelBase.LevelBase" 0))

(event Custom|InitcloudSpawner
  (Utilities|Time|SetTimerbyEvent (delegate Custom|SpawnCloud) (Math|Random|RandomFloatinRange 0.25 2.0) true))

(fn ConstructionScript
  (Components|Box|SetBoxExtent (Variables|Default|GetCloudSpawnZone) (Variables|Default|GetIn%20Box%20Extent) true))